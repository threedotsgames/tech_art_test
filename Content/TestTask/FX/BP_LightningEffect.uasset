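; Lightning effect actor that drives a Niagara bolt system toward the bounds of a target actor.
; Each tick, it computes the target's bounding-box corners from an offset array and keys them by distance to its own location.
; It sorts the distances and picks the nearest NumPoints corners as beam endpoints.
; It feeds all corners, those endpoints and the beam color, density, tiling, jitter and width settings into Niagara.
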(event `self.ReceiveTick`
  (params (DeltaSeconds :type "Float (single-precision)"))
  (bind _ns_lightningbolts (`self.NS_LightningBolts`))
  (bind (_origin _boxextent) (`self.GetActorBounds` (`self.TargetActor`) false false))
  (bind (_allcorners _beampoints) (`self.GetBoundsCorners` _origin _boxextent))
  (`NiagaraDataInterfaceArrayFunctionLibrary.SetNiagaraArrayPosition` _ns_lightningbolts "CornerPoints" _allcorners)
  (`NiagaraDataInterfaceArrayFunctionLibrary.SetNiagaraArrayPosition` _ns_lightningbolts "BeamEndPoints" _beampoints)
  (`NiagaraComponent.SetVariableLinearColor` _ns_lightningbolts "ColorMax" (`self.BeamColorMax`))
  (`NiagaraComponent.SetVariableLinearColor` _ns_lightningbolts "ColorMin" (`self.BeamColorMin`))
  (`NiagaraComponent.SetVariableFloat` _ns_lightningbolts "BeamDensity" (`self.BeamDensity`))
  (`NiagaraComponent.SetVariableFloat` _ns_lightningbolts "BeamTiling" (`self.BeamTiling`))
  (`NiagaraComponent.SetVariableFloat` _ns_lightningbolts "BeamJitterAmmount" (`self.BeamJitter`))
  (`NiagaraComponent.SetVariableFloat` _ns_lightningbolts "BeamWidth" (`self.BeamWidth`)))

(fn `GetBoundsCorners`
  (params (Origin :type "Vector Structure") (Extents :type "Vector Structure"))
  (returns (AllCorners :type "Array of Vector Structure") (BeamPoints :type "Array of Vector Structure"))
  (locals (Offsets :type "Array of Vector Structure") (Points :type "Map of Float (double-precision) to Vector Structure") (BeamTargetPoints :type "Array of Vector Structure") (dist :type "Array of Float (double-precision)"))
  ; clear arrays
  (`BlueprintMapLibrary.Map_Clear` (`local.Points`))
  (`KismetArrayLibrary.Array_Clear` (`local.BeamTargetPoints`))
  (`KismetArrayLibrary.Array_Clear` (`local.dist`))
  ; find all corners and distances to the beam start
  (for _array_element (`local.Offsets`)
    (bind _returnvalue (+ Origin (* _array_element Extents)))
    (`BlueprintMapLibrary.Map_Add` (`local.Points`) (`KismetMathLibrary.Vector_Distance` _returnvalue (`self.K2_GetActorLocation`)) _returnvalue))
  ; save distances to array and sort
  (bind _keys (`BlueprintMapLibrary.Map_Keys` (`local.Points`)))
  (bind _output_get (set `local.dist` _keys))
  (`KismetArrayLibrary.SortFloatArray` _output_get)
  ; loop through the distance array and add the vectors
  (for (_array_element_2 _array_index) _output_get
    (if (> _array_index (- (`self.NumPoints`) 1))
      (break)
      (else
        (`KismetArrayLibrary.Array_Add` (`local.BeamTargetPoints`) (`BlueprintMapLibrary.Map_Find` (`local.Points`) _array_element_2)))))
  (bind _values (`BlueprintMapLibrary.Map_Values` (`local.Points`)))
  (return _values (`local.BeamTargetPoints`)))

(fn `UserConstructionScript`)